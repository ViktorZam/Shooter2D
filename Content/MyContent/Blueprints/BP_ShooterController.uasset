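; Player controller for a 2D side-scroller that lets the player rotate the world in quarter turns with E and quit with Escape.
; On BeginPlay it caches the pawn and BP_RotateActor, then attaches ledges overlapping that actor's box to it.
; The RotateWorld timeline drives the actor's pitch from an accumulated angle, carrying attached ledges along, while a flag blocks input mid-turn.
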(event `self.ReceiveBeginPlay`
  (bind _as2dside_scroller_character (cast `/Game/2DSideScrollerBP/Blueprints/2DSideScrollerCharacter` (`self.K2_GetPawn`)))
  (set `self.CharacterRef` _as2dside_scroller_character)
  (bind _returnvalue (`GameplayStatics.GetActorOfClass` "/Game/MyContent/Blueprints/BP_RotateActor.BP_RotateActor_C"))
  (bind _output_get (set `self.RotateActorRef` _returnvalue))
  (for _array_element (`PrimitiveComponent.GetOverlappingActors` (`/Game/MyContent/Blueprints/BP_RotateActor.Box` _output_get) "/Game/MyContent/Blueprints/BP_Ledge.BP_Ledge_C")
    (`self.K2_AttachToActor` _array_element (`self.RotateActorRef`) "None" "KeepWorld" "KeepWorld" "KeepWorld" true)))

(event `Key|Escape`
  (params (Key :type "Key Structure"))
  (:`Pressed`
    (`KismetSystemLibrary.QuitGame` null "Quit")))

(event `Key|E`
  (params (Key :type "Key Structure"))
  (:`Pressed`
    ;[1 1 1] RotateWorld
    (if (not (`self.WorldIsRotate?`))
      (if (== (`self.CurrentRotationSceneY`) 360.0)
        (set `self.CurrentRotationSceneY` 0.0))
      (set `self.WorldIsRotate?` true)
      (bind (_direction _degrees) (`Timeline|RotateWorld` :!via `PlayFromStart`)
        (:`Update`
          (`self.K2_SetActorRelativeRotation` (`self.RotateActorRef`) (`KismetMathLibrary.MakeRotator` 0.0 (+ _degrees (`self.CurrentRotationSceneY`))) false false))
        (:`Finished`
          (set `self.WorldIsRotate?` false)
          (set `self.CurrentRotationSceneY` (+ (`self.CurrentRotationSceneY`) 90.0)))))))

(fn `UserConstructionScript`)