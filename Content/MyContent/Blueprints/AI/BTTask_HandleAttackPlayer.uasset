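; Behavior Tree task that makes an AI enemy attack the player character when it is directly ahead.
; It runs a forward object trace for pawns from the controlled pawn and calls AttackPlayer on the enemy character if the trace hits the side-scroller character.
; Whether the trace hits the player or not, it then sets the IsReload blackboard flag and finishes successfully.
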(event `self.ReceiveExecuteAI`
  (params (OwnerController :type "AIController Object Reference") (ControlledPawn :type "Pawn Object Reference"))
  (bind _returnvalue (`Actor.K2_GetActorLocation` ControlledPawn))
  (bind _outhit (`KismetSystemLibrary.LineTraceSingleForObjects` _returnvalue (+ _returnvalue (* (`KismetMathLibrary.GetForwardVector` (`Actor.K2_GetActorRotation` ControlledPawn)) 800.0)) (`|MakeArray` "ObjectTypeQuery3" :!type "EObjectTypeQuery Enum") false (`|MakeArray` ControlledPawn :!type "Actor Object Reference")))
  (cast `/Game/2DSideScrollerBP/Blueprints/2DSideScrollerCharacter` (`.HitActor` (`GameplayStatics.BreakHitResult` _outhit))
    (:`then`
      (bind _asbp_aienemu_character (cast `/Game/2DSideScrollerBP/Blueprints/BP_AIEnemuCharacter` ControlledPawn))
      (`/Game/2DSideScrollerBP/Blueprints/BP_AIEnemuCharacter.AttackPlayer` _asbp_aienemu_character))
    (:`CastFailed`
      _))
  (`BTFunctionLibrary.SetBlackboardValueAsBool` (`self.IsReload`) true)
  (`self.FinishExecute` true))