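; Behavior tree task that steers a BP_AIEnemuCharacter toward the actor stored in the PlayerRef blackboard key.
; On AI tick it sets the pawn's yaw to face that actor, then adds movement input using only the X component of its forward vector, without navigation pathfinding.
; It then finishes as failed, so each execution performs a single steering step.
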(event `self.ReceiveTickAI`
  (params (OwnerController :type "AIController Object Reference") (ControlledPawn :type "Pawn Object Reference") (DeltaSeconds :type "Float (single-precision)"))
  (bind _returnvalue_x (`KismetMathLibrary.BreakVector` (`KismetMathLibrary.GetForwardVector` (`Actor.K2_GetActorRotation` (`self.ControlledPawn`)))))
  (bind _asbp_aienemu_character (cast `/Game/2DSideScrollerBP/Blueprints/BP_AIEnemuCharacter` ControlledPawn))
  (bind _output_get (set `self.ControlledPawn` _asbp_aienemu_character))
  (bind (_returnvalue_roll _returnvalue_pitch _returnvalue_yaw) (`KismetMathLibrary.BreakRotator` (`KismetMathLibrary.FindLookAtRotation` (`Actor.K2_GetActorLocation` _output_get) (`Actor.K2_GetActorLocation` (`BTFunctionLibrary.GetBlackboardValueAsActor` (`self.PlayerRef`))))))
  (`Actor.K2_SetActorRotation` (`self.ControlledPawn`) (`KismetMathLibrary.MakeRotator` 0.0 0.0 _returnvalue_yaw) false)
  (`Pawn.AddMovementInput` (`self.ControlledPawn`) (`KismetMathLibrary.MakeVector` _returnvalue_x) 1.0 false)
  (`self.FinishExecute` false))